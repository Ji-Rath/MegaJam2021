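; Player controller that adds the main UI at BeginPlay and handles the game-over sequence.
; CallGameOver clears the inventory component of the level's BP_Storage actor when the run is not successful.
; On either outcome it then shows the game-over widget and sets the time-elapsed state on BP_MainGameMode.
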(event EventBeginPlay
  (bind _returnvalue (UserInterface|CreateWidget "/BasicUI/Widget_MainUI.Widget_MainUI_C" self))
  (UserInterface|Viewport|AddtoViewport _returnvalue 0))

(fn ConstructionScript)

(fn CallGameOver
  (params (bSuccess :type Boolean))
  (bind _returnvalue (Actor|GetActorOfClass "/Game/Blueprints/InteractableObjects/BP_Storage.BP_Storage_C"))
  (if bSuccess
    _
    (else
      (Utilities|Array|Clear (Variables|/Script/MegaJam2021.InventoryComponent|GetInventory (Actor|GetComponentbyClass _returnvalue "/Game/Blueprints/BPC_Inventory.BPC_Inventory_C")))))
  (bind _returnvalue_2 (UserInterface|CreateWidget "/Game/Blueprints/UI/Widget_GameOver.Widget_GameOver_C" self))
  (UserInterface|Viewport|AddtoViewport _returnvalue_2 0)
  (bind _asbp_main_game_mode (Utilities|Casting|CastToBP_MainGameMode (Game|GetGameMode)))
  (Default|SetTimeElapsedState _asbp_main_game_mode true))