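; Main game mode that tracks elapsed play time and runs a level-wide lockdown.
; A looping one-second timer increments the elapsed time and can be paused or resumed.
; Lockdown sets the state of every DoorOpen actor and recolours all spot lights between pale blue and red.
; Ending a lockdown starts a 30-second cooldown before lockdown can be triggered again.
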(event EventBeginPlay
  (Utilities|Time|SetTimerbyFunctionName 0 "IncrementTime" 1.0 true))

(fn ConstructionScript)

(fn SetLockdown
  (params (bEnableLockdown :type Boolean))
  (bind _returnvalue (not bEnableLockdown))
  (if (Variables|Default|GetbCanStartLockdown)
    (CallFunction|SetDoorState _returnvalue)
    (CallFunction|SetLights _returnvalue)
    (bind _output_get (Variables|Default|SetbInLockdown bEnableLockdown))
    (if (not _output_get)
      (Variables|Default|SetbCanStartLockdown false)
      (Utilities|Time|SetTimerbyFunctionName 0 "ClearLockdownCooldown" 3e+01))))

(fn IncrementTime
  (Math|Float|IncrementFloat (Variables|Default|GetTimeElapsed)))

(fn SetTimeElapsedState
  (params (bPaused :type Boolean))
  (if bPaused
    (Utilities|Time|ClearTimerbyFunctionName 0 "IncrementTime")
    (else
      (Utilities|Time|SetTimerbyFunctionName 0 "IncrementTime" 1.0 true))))

(fn ClearLockdownCooldown
  (Variables|Default|SetbCanStartLockdown true))

(fn SetDoorState
  (params (bOpen :type Boolean))
  (bind _outactors (Actor|GetAllActorsOfClass "/Game/Blueprints/InteractableObjects/DoorOpen.DoorOpen_C"))
  (for _array_element _outactors
    (Default|SetDoorState _array_element bOpen)))

(fn SetLights
  (params (Condition :type Boolean))
  (bind _outactors (Actor|GetAllActorsOfClass "/Script/Engine.SpotLight"))
  (for _array_element _outactors
    (if Condition
      (Rendering|Components|Light|SetLightColor (Variables|/Script/Engine.SpotLight|GetSpotLightComponent _array_element) "(R=0.631373,G=0.666667,B=1.000000,A=1.000000)" true)
      (else
        (Rendering|Components|Light|SetLightColor (Variables|/Script/Engine.SpotLight|GetSpotLightComponent _array_element) "(R=0.572917,G=0.190972,B=0.190972,A=1.000000)" true)))))