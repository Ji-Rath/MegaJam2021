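; Interactable trap that the player disarms by holding PickUp/Interact inside its box, where a DisarmTrap widget is shown.
; A Gate and DoOnce on the input axis time the hold, then after a delay flag the trap Destroyed and destroy it.
; Releasing the key also destroys the actor.
; Ending overlap removes the widget and, unless Destroyed is set, sends a referenced pawn toward the player via AIMoveTo.
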(event OnComponentBeginOverlap(Box)
  (params (OverlappedComponent :type Primitive%20Component%20Object%20Reference) (OtherActor :type Actor%20Object%20Reference) (OtherComp :type Primitive%20Component%20Object%20Reference) (OtherBodyIndex :type Integer) (bFromSweep :type Boolean) (SweepResult :type Hit%20Result%20Structure%20%28by%20ref%29))
  (Input|EnableInput (Game|GetPlayerController 0))
  (Utilities|Casting|CastToBP_Player OtherActor)
  (bind _returnvalue (UserInterface|CreateWidget "/Game/Blueprints/UI/DisarmTrap.DisarmTrap_C"))
  (UserInterface|Viewport|AddtoViewport _returnvalue 0))

(event OnComponentEndOverlap(Box)
  (params (OverlappedComponent :type Primitive%20Component%20Object%20Reference) (OtherActor :type Actor%20Object%20Reference) (OtherComp :type Primitive%20Component%20Object%20Reference) (OtherBodyIndex :type Integer))
  (Input|DisableInput (Game|GetPlayerController 0))
  (bind _asbp_player (Utilities|Casting|CastToBP_Player OtherActor))
  (Widget|RemovefromParent (stale OnComponentBeginOverlap(Box) _returnvalue))
  (if (not (Variables|Default|GetDestroyed?))
    (AI|AIMoveTo (Variables|Default|GetPawn) "0, 0, 0" _asbp_player 5.0 false)))

(event EventBeginPlay)

(event Collision|EventActorBeginOverlap
  (params (OtherActor :type Actor%20Object%20Reference)))

(event EventTick
  (params (DeltaSeconds :type Float%20%28single-precision%29)))

(event Input|ActionEvents|InputActionPickUp/Interact
  (params (Key :type Key%20Structure))
  (:Pressed
    (Utilities|FlowControl|Gate true) ; enters at Open
  )
  (:Released
    (Utilities|FlowControl|Sequence
      (:then_0
        (Utilities|FlowControl|Gate true) ; enters at Close
      )
      (:then_1
        (Utilities|FlowControl|DoOnce false) ; enters at Reset
      )
      (:then_2
        (Actor|DestroyActor)
        (Variables|Default|SetDestroyed? false)))))

(event Input|AxisEvents|InputAxisPickUp/Interact
  (params (AxisValue :type Float%20%28single-precision%29))
  (Utilities|FlowControl|Gate true
    (:Exit
      (if (>= (Class|PlayerController|GetInputKeyTimeDown (Game|GetPlayerController 0) (stale Input|ActionEvents|InputActionPickUp/Interact Key)) 2.0)
        (Utilities|FlowControl|DoOnce false
          (:Completed
            (Utilities|FlowControl|Delay 3.0)
            (Variables|Default|SetDestroyed? true)
            (Actor|DestroyActor)))))))

(fn ConstructionScript)