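; Interactable button that toggles every door in its DoorList, or lifts lockdown instead when the main game mode is in lockdown.
; Box overlap tracks PlayerOverlapping and shows or removes the Door prompt widget, without filtering the overlapping actor.
; Action starts a timed cooldown and hides the prompt, which returns when the cooldown clears if the overlap persists.
; Input enable/disable code in PlayerEnter and PlayerLeave is disconnected.
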(event OnComponentBeginOverlap(Box)
  (params (OverlappedComponent :type Primitive%20Component%20Object%20Reference) (OtherActor :type Actor%20Object%20Reference) (OtherComp :type Primitive%20Component%20Object%20Reference) (OtherBodyIndex :type Integer) (bFromSweep :type Boolean) (SweepResult :type Hit%20Result%20Structure%20%28by%20ref%29))
  (Variables|Default|SetbPlayerOverlapping true)
  (CallFunction|PlayerEnter OtherActor))

(event OnComponentEndOverlap(Box)
  (params (OverlappedComponent :type Primitive%20Component%20Object%20Reference) (OtherActor :type Actor%20Object%20Reference) (OtherComp :type Primitive%20Component%20Object%20Reference) (OtherBodyIndex :type Integer))
  (Variables|Default|SetbPlayerOverlapping false)
  (CallFunction|PlayerLeave OtherActor))

(event EventAction
  (if (Variables|Default|GetbCanInteract)
    (bind _asbp_main_game_mode (Utilities|Casting|CastToBP_MainGameMode (Game|GetGameMode)))
    (if (Variables|/Game/Blueprints/PlayerFiles/BP_MainGameMode.BP_MainGameMode_C|GetbInLockdown _asbp_main_game_mode)
      (Default|SetLockdown _asbp_main_game_mode false) ; Disable lockdown if it was enabled
      (else
        (for _array_element (Variables|Default|GetDoorList)
          (Default|ToggleDoor _array_element) ; Normal toggle door logic
        )))
    (Utilities|Time|SetTimerbyFunctionName 0 "ClearButtonCooldown" (Variables|Default|GetButtonCooldown)) ; Begin button cooldown
    (Variables|Default|SetbCanInteract false)
    (CallFunction|PlayerLeave (Game|Player|GetPlayerPawn 0))))

(event Input|ActionEvents|InputActionPickUp/Interact
  (params (Key :type Key%20Structure :default "None")))

(fn ConstructionScript)

(fn ClearButtonCooldown
  (Variables|Default|SetbCanInteract true)
  (if (Variables|Default|GetbPlayerOverlapping)
    (CallFunction|PlayerEnter (Game|Player|GetPlayerPawn 0))))

(fn PlayerLeave
  (params (Player :type Actor%20Object%20Reference))
  (Widget|RemovefromParent (Variables|Default|GetWidgetReference)))

(fn PlayerEnter
  (params (Player :type Actor%20Object%20Reference))
  (if (Variables|Default|GetbCanInteract)
    (bind _returnvalue (UserInterface|CreateWidget "/Game/Blueprints/UI/Door.Door_C"))
    (UserInterface|Viewport|AddtoViewport _returnvalue 0)
    (Variables|Default|SetWidgetReference _returnvalue)))