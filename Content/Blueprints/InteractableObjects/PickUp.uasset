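; Pickup actor that the player collects into an inventory-style component with the PickUp/Interact action.
; Box overlap enables input for any actor, but shows the Interactable widget only for BP_Player; end overlap reverses both.
; Pressing the action calls DestroyActor, then passes ItemData to TryAddItem on the player character's component and prints the result, so the pickup is destroyed even if adding fails.
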(event OnComponentBeginOverlap(Box)
  (params (OverlappedComponent :type Primitive%20Component%20Object%20Reference) (OtherActor :type Actor%20Object%20Reference) (OtherComp :type Primitive%20Component%20Object%20Reference) (OtherBodyIndex :type Integer) (bFromSweep :type Boolean) (SweepResult :type Hit%20Result%20Structure%20%28by%20ref%29))
  (Input|EnableInput (Game|GetPlayerController 0))
  (Utilities|Casting|CastToBP_Player OtherActor)
  (bind _returnvalue (UserInterface|CreateWidget "/Game/Blueprints/UI/Interactable.Interactable_C"))
  (UserInterface|Viewport|AddtoViewport _returnvalue 0))

(event OnComponentEndOverlap(Box)
  (params (OverlappedComponent :type Primitive%20Component%20Object%20Reference) (OtherActor :type Actor%20Object%20Reference) (OtherComp :type Primitive%20Component%20Object%20Reference) (OtherBodyIndex :type Integer))
  (Input|DisableInput (Game|GetPlayerController 0))
  (Utilities|Casting|CastToBP_Player OtherActor)
  (Widget|RemovefromParent (stale OnComponentBeginOverlap(Box) _returnvalue)))

(event EventBeginPlay)

(event Collision|EventActorBeginOverlap
  (params (OtherActor :type Actor%20Object%20Reference)))

(event EventTick
  (params (DeltaSeconds :type Float%20%28single-precision%29)))

(event Input|ActionEvents|InputActionPickUp/Interact
  (params (Key :type Key%20Structure :default "None"))
  (:Pressed
    (Actor|DestroyActor)
    (bind _returnvalue (CallFunction|TryAddItem (Actor|GetComponentbyClass (Game|GetPlayerCharacter 0) 0) (.ItemData (Variables|Default|GetItemData))))
    (Development|PrintString (Utilities|String|ToString(Boolean) _returnvalue))))

(fn ConstructionScript)