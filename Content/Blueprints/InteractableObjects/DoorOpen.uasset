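; Interactable door that slides its mesh between closed and open positions.
; SetDoorState stores the DoorOpen flag and plays or reverses the Door timeline, whose output scaled by Height sets the mesh's relative location.
; ToggleDoor flips the current state through SetDoorState, and BeginPlay animates the door open if DoorOpen is already set.
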(event Custom|SetDoorState
  (params (bOpen :type Boolean))
  (if bOpen
    (Variables|Default|SetbDoorOpen true)
    (bind _door (Timeline|Door Play)
      (:Update
        (Transformation|SetRelativeLocation (Variables|Default|GetDoorMesh) (Math|Conversions|ToVector(Float) (* _door (Variables|Default|GetHeight))) false false)))
    (else
      (Variables|Default|SetbDoorOpen false)
      (Timeline|Door Reverse))))

(event Custom|ToggleDoor
  (CallFunction|SetDoorState (not (Variables|Default|GetbDoorOpen))))

(event Collision|EventActorBeginOverlap
  (params (OtherActor :type Actor%20Object%20Reference)))

(event EventTick
  (params (DeltaSeconds :type Float%20%28single-precision%29)))

(event EventBeginPlay
  (if (Variables|Default|GetbDoorOpen)
    (CallFunction|SetDoorState true)))

(fn ConstructionScript)