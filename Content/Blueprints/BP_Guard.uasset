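; Guard enemy pawn driven by a Behavior Tree, with a patrol reference, a configurable idle behavior and a text readout of its AI state.
; On BeginPlay it writes the patrol reference to the SplineReference blackboard key and injects its idle behavior asset as a dynamic subtree.
; When possessed by a BP_EnemyController, it binds to that controller's state update event and shows the enemy state name on its TextRender.
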(event Custom|OnStateUpdated
  (params (EnemyState :type EEnemyState%20Enum :default "Idle"))
  (Rendering|Components|TextRender|SetText (Variables|Default|GetTextRender) (Utilities|Text|ToText(String) (Utilities|String|EnumtoString EnemyState))))

(event EventBeginPlay
  (|CallParentFunction)
  (AI|Components|Blackboard|SetValueasObject (AI|GetBlackboard 0) (Utilities|Name|MakeLiteralName "SplineReference") (Variables|Default|GetPatrolReference))
  (Class|BehaviorTreeComponent|SetDynamicSubtree (Actor|GetComponentbyClass (Pawn|GetController) "/Script/AIModule.BehaviorTreeComponent") "(TagName=\"IdleBehavior\")" (Variables|Default|GetIdleBehavior)))

(event EventPossessed
  (params (NewController :type Controller%20Object%20Reference))
  (|CallParentFunction NewController)
  (bind _asbp_enemy_controller (Utilities|Casting|CastToBP_EnemyController NewController))
  (EventDispatchers|AssignOnStateUpdated _asbp_enemy_controller (EventDispatchers|CreateEvent :!event Custom|OnStateUpdated)))

(fn ConstructionScript)