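; Behavior tree task that turns the AI pawn to face the actor stored in a Blackboard key.
; On execute it computes a yaw-only look-at rotation toward that actor once, so the target's later movement is not tracked.
; Each tick it interpolates the pawn's rotation toward that yaw at a configurable speed and finishes successfully once within a small tolerance.
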(event EventReceiveExecuteAI
  (params (OwnerController :type AI%20Controller%20Object%20Reference) (ControlledPawn :type Pawn%20Object%20Reference))
  (Variables|Default|SetTargetRotation (Math|Rotator|MakeRotator 0.0 0.0 (.yaw (Math|Rotator|FindLookatRotation (Transformation|GetActorLocation ControlledPawn) (Transformation|GetActorLocation (AI|BehaviorTree|GetBlackboardValueasActor (Variables|Default|GetTarget))))))))

(event EventReceiveTickAI
  (params (OwnerController :type AI%20Controller%20Object%20Reference) (ControlledPawn :type Pawn%20Object%20Reference) (DeltaSeconds :type Float%20%28single-precision%29))
  (bind _returnvalue (Transformation|GetActorRotation ControlledPawn))
  (bind _targetrotation (Variables|Default|GetTargetRotation))
  (bind _interpspeed (Variables|Default|GetInterpSpeed))
  (bind _returnvalue_2 (Math|Interpolation|RInterpTo _returnvalue _targetrotation DeltaSeconds _interpspeed))
  (Transformation|SetActorRotation ControlledPawn _returnvalue_2)
  (if (Math|Rotator|Equal(Rotator) _returnvalue_2 (Variables|Default|GetTargetRotation) 1e+01)
    (AI|BehaviorTree|FinishExecute true)))