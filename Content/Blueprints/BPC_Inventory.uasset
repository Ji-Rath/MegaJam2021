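; Inventory component that provides the on-screen UI for the inventory of a player-controlled pawn.
; On BeginPlay it creates the inventory widget for the owner's player controller, passes in the inventory size and adds it to the viewport.
; The SpawnWidgetItem override calls its parent, then adds an item widget to the inventory overlay.
; Items are placed by render translation on a 100-unit grid, with Position X and Y swapped.
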(event EventBeginPlay
  (|CallParentFunction)
  (bind _aspawn (Utilities|Casting|CastToPawn (Components|GetOwner)))
  (bind _asplayer_controller (Utilities|Casting|CastToPlayerController (Pawn|GetController _aspawn)))
  (bind _returnvalue (UserInterface|CreateWidget "/Game/Blueprints/UI/Inventory/Widget_Inventory.Widget_Inventory_C" _asplayer_controller (Variables|Default|GetInventorySize)))
  (UserInterface|Viewport|AddtoViewport _returnvalue 0)
  (Variables|Default|SetInventoryWidget _returnvalue))

(event EventSpawnWidgetItem
  (params (Item :type Item%20Data%20Object%20Reference) (Position :type Int%20Vector%202D%20Structure))
  (bind (_x _y) (Utilities|Struct|BreakIntVector2D Position))
  (|CallParentFunction Item Position)
  (bind _returnvalue (UserInterface|CreateWidget "/Game/Blueprints/UI/Inventory/Widget_InventoryItem.Widget_InventoryItem_C" 0 Item))
  (Class|Overlay|AddChildtoOverlay (Variables|/Game/Blueprints/UI/Inventory/Widget_Inventory.Widget_Inventory_C|GetOverlay_20 (Variables|Default|GetInventoryWidget)) _returnvalue)
  (Class|Widget|SetRenderTranslation _returnvalue (Math|Vector2D|MakeVector2D (* _y 1e+02) (* _x 1e+02))))